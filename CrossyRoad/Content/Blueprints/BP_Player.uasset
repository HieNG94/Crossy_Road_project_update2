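; BP_Player is a player Character that moves in hops along world axes, like a step-based mover.
; Forward, right and backward input each snap the mesh's yaw, launch the character with an upward boost, then disable input for a delay.
; The left-hop logic and an offset-based movement snippet are present but unwired.
; Tick prints the actor location for debugging, and the forward hop also prints it after its delay.
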(event `self.ReceiveTick`
  (params (DeltaSeconds :type "Float (single-precision)"))
  (`KismetSystemLibrary.PrintString` (`KismetStringLibrary.Conv_VectorToString` (`self.K2_GetActorLocation`)) :!label _label))

(event `InputAction|MoveForward`
  (params (Key :type "Key Structure"))
  ;[1 1 1] Move forward
  (:`Pressed`
    (`SceneComponent.K2_SetWorldRotation` :`self` (`self.Mesh`))
    (`self.LaunchCharacter` (+ (`MovementComponent.Velocity` (`self.CharacterMovement`)) (`KismetMathLibrary.MakeVector` (`self.MoveSpeed`) 0.0 200.0)) true true)
    (`self.DisableInput` null)
    (`KismetSystemLibrary.Delay` (`self.DelayInput`))
    (`self.EnableInput` null)
    (goto _label)))

(event `InputAction|MoveRight`
  (params (Key :type "Key Structure"))
  ;[1 1 1] Move right
  (:`Pressed`
    (`SceneComponent.K2_SetWorldRotation` (`self.Mesh`) (struct :`Yaw` 90.0) false false)
    (`self.LaunchCharacter` (+ (`MovementComponent.Velocity` (`self.CharacterMovement`)) (`KismetMathLibrary.MakeVector` 0.0 (`self.MoveSpeed`) 200.0)) true true)
    (`self.DisableInput` null)
    (`KismetSystemLibrary.Delay` (`self.DelayInput`))
    (`self.EnableInput` null)))

(event `InputAction|MoveBackward`
  (params (Key :type "Key Structure"))
  ;[1 1 1] Move backward
  (:`Pressed`
    (`SceneComponent.K2_SetWorldRotation` (`self.Mesh`) (struct :`Yaw` 180.0) false false)
    (`self.LaunchCharacter` (+ (`MovementComponent.Velocity` (`self.CharacterMovement`)) (`KismetMathLibrary.MakeVector` (* (`self.MoveSpeed`) -1.0) 0.0 200.0)) true true)
    (`self.DisableInput` null)
    (`KismetSystemLibrary.Delay` (`self.DelayInput`))
    (`self.EnableInput` null)))

(event `InputAction|MoveLeft`
  (params (Key :type "Key Structure"))
  ;[1 1 1] Move left
)

(fn `UserConstructionScript`)