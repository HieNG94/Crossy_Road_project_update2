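; BP_Map is a map actor that recycles traffic vehicles as they leave its left and right trigger zones.
; When a BP_Car or BP_Truck stops overlapping either zone, it is destroyed and a new one of the same class spawns at a fixed, hard-coded transform.
; Trucks respawn at a different position and facing per zone, while cars from both zones return to nearly the same spot facing the same way.
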(event `self.TriggerZoneRight.OnComponentEndOverlap`
  (params (OverlappedComponent :type "PrimitiveComponent Object Reference") (OtherActor :type "Actor Object Reference") (OtherComp :type "PrimitiveComponent Object Reference") (OtherBodyIndex :type Integer))
  (`|ExecutionSequence`
    (:`then_0`
      (bind _asbp_car (cast `/Game/Blueprints/BP_Car` OtherActor))
      (`self.K2_DestroyActor` _asbp_car)
      (`|SpawnActorFromClass` "/Game/Blueprints/BP_Car.BP_Car_C" (`KismetMathLibrary.MakeTransform` (-240.0 -630.0 35.0) (struct :`Yaw` 90.0)) "Undefined" "OverrideRootScale" null null))
    (:`then_1`
      (bind _asbp_truck (cast `/Game/Blueprints/BP_Truck` OtherActor))
      (`self.K2_DestroyActor` _asbp_truck)
      (`|SpawnActorFromClass` "/Game/Blueprints/BP_Truck.BP_Truck_C" (`KismetMathLibrary.MakeTransform` (70.0 -790.0 0.0) (struct :`Yaw` 90.0)) "Undefined" "OverrideRootScale" null null))))

(event `self.TriggerZoneLeft.OnComponentEndOverlap`
  (params (OverlappedComponent :type "PrimitiveComponent Object Reference") (OtherActor :type "Actor Object Reference") (OtherComp :type "PrimitiveComponent Object Reference") (OtherBodyIndex :type Integer))
  (`|ExecutionSequence`
    (:`then_0`
      (bind _asbp_car (cast `/Game/Blueprints/BP_Car` OtherActor))
      (`self.K2_DestroyActor` _asbp_car)
      (`|SpawnActorFromClass` "/Game/Blueprints/BP_Car.BP_Car_C" (`KismetMathLibrary.MakeTransform` (-240.0 -630.0 40.0) (struct :`Yaw` 90.0)) "Undefined" "OverrideRootScale" null null))
    (:`then_1`
      (bind _asbp_truck (cast `/Game/Blueprints/BP_Truck` OtherActor))
      (`self.K2_DestroyActor` _asbp_truck)
      (`|SpawnActorFromClass` "/Game/Blueprints/BP_Truck.BP_Truck_C" (`KismetMathLibrary.MakeTransform` (-250.0 790.0 0.0) (struct :`Yaw` -90.0)) "Undefined" "OverrideRootScale" null null))))

(fn `UserConstructionScript`)